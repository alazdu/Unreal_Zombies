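; Test cube actor that spins around its vertical axis and reports trigger box overlaps on the player's HUD.
; Tick calls SpinEvent, which adds a fixed yaw step each frame while IsSpinning is true; the nodes toggling that flag are disconnected.
; Box begin and end overlaps cast to ThirdPersonCharacter and overwrite the HUD health text with enter/exit messages, the exit reusing the begin-overlap cast result.
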(event OnComponentEndOverlap(Box)
  (params (OverlappedComponent :type Primitive%20Component%20Object%20Reference) (OtherActor :type Actor%20Object%20Reference) (OtherComp :type Primitive%20Component%20Object%20Reference) (OtherBodyIndex :type Integer))
  (Utilities|Casting|CastToThirdPersonCharacter OtherActor)
  (Rendering|Components|TextRender|SetText (Variables|/Game/Zombies/Blueprints/Zombie_HUD.Zombie_HUD_C|GetHealthValue (Variables|/Game/ThirdPersonBP/Blueprints/ThirdPersonCharacter.ThirdPersonCharacter_C|GetHUDReference (stale OnComponentBeginOverlap(Box) _asthird_person_character))) "Saloi"))

(event OnComponentBeginOverlap(Box)
  (params (OverlappedComponent :type Primitive%20Component%20Object%20Reference) (OtherActor :type Actor%20Object%20Reference) (OtherComp :type Primitive%20Component%20Object%20Reference) (OtherBodyIndex :type Integer) (bFromSweep :type Boolean) (SweepResult :type Hit%20Result%20Structure%20%28by%20ref%29))
  (bind _asthird_person_character (Utilities|Casting|CastToThirdPersonCharacter OtherActor))
  (Rendering|Components|TextRender|SetText (Variables|/Game/Zombies/Blueprints/Zombie_HUD.Zombie_HUD_C|GetHealthValue (Variables|/Game/ThirdPersonBP/Blueprints/ThirdPersonCharacter.ThirdPersonCharacter_C|GetHUDReference _asthird_person_character)) "Entro"))

(event Custom|SpinEvent
  (if (Variables|Default|GetIsSpinning)
    (Transformation|SetActorRotation (Math|Rotator|MakeRotator 0.0 0.0 (+ (.Yaw (Math|Rotator|BreakRotator (Transformation|GetActorRotation))) 1.0)))))

(event EventBeginPlay)

(event Collision|EventActorBeginOverlap
  (params (OtherActor :type Actor%20Object%20Reference)))

(event EventTick
  (params (DeltaSeconds :type Float%20%28single-precision%29))
  (CallFunction|SpinEvent))

(fn ConstructionScript)