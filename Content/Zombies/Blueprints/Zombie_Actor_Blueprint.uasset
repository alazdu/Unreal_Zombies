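; Zombie enemy actor that roams around its spawn point, chases the player once detected and attacks at close range.
; Box overlaps notify the animation Blueprint, whose PlayerDetected and IsChasing flags select the behavior in Tick.
; Movement uses per-frame SetActorLocation steps on XY without sweep; timeline and look-at rotation nodes are disconnected.
; Attacks use delays to time health loss and cooldown, and FinishGame halts the behavior.
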(event OnComponentBeginOverlap(Box)
  (params (OverlappedComponent :type Primitive%20Component%20Object%20Reference) (OtherActor :type Actor%20Object%20Reference) (OtherComp :type Primitive%20Component%20Object%20Reference) (OtherBodyIndex :type Integer) (bFromSweep :type Boolean) (SweepResult :type Hit%20Result%20Structure%20%28by%20ref%29))
  ;[1 1 1] El jugador entra en el área del zombie.
  (Utilities|Casting|CastToThirdPersonCharacter OtherActor)
  (Development|PrintString "El jugador es visible." false)
  (Default|DetectPlayer (Variables|Default|GetAnimationReference)))

(event OnComponentEndOverlap(Box)
  (params (OverlappedComponent :type Primitive%20Component%20Object%20Reference) (OtherActor :type Actor%20Object%20Reference) (OtherComp :type Primitive%20Component%20Object%20Reference) (OtherBodyIndex :type Integer))
  ;[1 1 1] El jugador sale del área del zombie y ya no es detectado.
  (Utilities|Casting|CastToThirdPersonCharacter OtherActor)
  (Development|PrintString "El jugador ya no es visible" false)
  (Default|LosePlayer (Variables|Default|GetAnimationReference)))

(event Custom|FinishGame
  ;[1 1 1] Finish Game
  (Variables|Default|SetisPlaying false)
  (Default|FinishGameFunction (Variables|Default|GetAnimationReference)))

(event EventBeginPlay
  ;[1 1 1] Guarda la referencia al componente de Animacion y guarda la posición Inicial del zombie
  (bind _output_get (Variables|Default|SetinitialPosition (Transformation|GetActorLocation)))
  (Development|PrintString (Utilities|String|ToString(Vector) _output_get) false)
  (bind _aszombie_animation_blueprint (Utilities|Casting|CastToZombieAnimationBlueprint (Components|SkeletalMesh|GetAnimInstance (Variables|SkeletalMeshActor|GetSkeletalMeshComponent)))
    (:then
      (bind _output_get_2 (Variables|Default|SetAnimationReference _aszombie_animation_blueprint))
      (Development|PrintString "Correcto anim" false)
      (Variables|/Game/Zombies/Blueprints/ZombieAnimationBlueprint.ZombieAnimationBlueprint_C|SetplayerDetected _output_get_2 false))
    (:CastFailed
      (Development|PrintString "Cast Failed for Animation BLueprint"))))

(event Collision|EventActorBeginOverlap
  (params (OtherActor :type Actor%20Object%20Reference)))

(event EventTick
  (params (DeltaSeconds :type Float%20%28single-precision%29))
  (bind _returnvalue (Transformation|GetActorLocation))
  (bind _returnvalue_2 (Transformation|GetActorLocation))
  (bind _returnvalue_3 (Transformation|GetActorLocation))
  (bind _player (Variables|Default|Getplayer))
  (bind _animationreference (Variables|Default|GetAnimationReference))
  (bind _player_2 (Variables|Default|Getplayer))
  (bind _speedchasing (Variables|Default|GetspeedChasing))
  (bind _returnvalue_4 (Transformation|GetActorLocation _player))
  (bind (_x _y) (Math|Vector|BreakVector _returnvalue))
  (bind _returnvalue_5 (Transformation|GetActorLocation _player_2))
  (bind (_x_2 _y_2) (Math|Vector|BreakVector _returnvalue_4))
  (bind _returnvalue_6 (Math|Vector|MakeVector _x _y 0.0))
  (bind _returnvalue_7 (- _returnvalue_5 _returnvalue_3))
  (bind _returnvalue_8 (Math|Vector|MakeVector _x_2 _y_2 0.0))
  (bind _returnvalue_9 (Math|Vector|Normalize _returnvalue_7))
  (bind _returnvalue_10 (Math|Vector|Distance(Vector) _returnvalue_6 _returnvalue_8))
  (bind _returnvalue_11 (* _returnvalue_9 _speedchasing))
  (bind (_x_3 _y_3) (Math|Vector|BreakVector _returnvalue_11))
  ;[1 1 1] Código para que le zombie deambule
  (if (Variables|Default|GetisPlaying)
    (if (Variables|/Game/Zombies/Blueprints/ZombieAnimationBlueprint.ZombieAnimationBlueprint_C|GetplayerDetected (Variables|Default|GetAnimationReference))
      ;[1 1 1] Chase Player
      (if (Variables|/Game/Zombies/Blueprints/ZombieAnimationBlueprint.ZombieAnimationBlueprint_C|GetisChasing _animationreference)
        (Development|PrintString (Utilities|String|ToString(Float) _returnvalue_10) false false)
        (if (< _returnvalue_10 175.0)
          (if (not (Variables|Default|GetisMakingDamage))
            (Default|DamagePlayer _animationreference)
            (Development|PrintString "DamagePlayer" false)
            (Variables|Default|SetisMakingDamage true)
            (Utilities|FlowControl|Delay 1.1)
            (Default|DecreaseHealth (Variables|Default|Getplayer))
            (Utilities|FlowControl|Delay 1.5)
            (Variables|Default|SetisMakingDamage false))
          (else
            (Default|StopDamagePlayer _animationreference)
            (Transformation|SetActorLocation (+ (Math|Vector|MakeVector _x_3 _y_3 0.0) _returnvalue_3) false false))))
      (else
        (bind _output_get (Variables|Default|SetcurrentIntervalIdle (+ DeltaSeconds (Variables|Default|GetcurrentIntervalIdle))))
        (Transformation|SetActorLocation (+ (Math|Vector|MakeVector (.X (Math|Vector|BreakVector (* (Math|Vector|Normalize (- (stale _output_get_3) _returnvalue_2)) (Variables|Default|GetspeedRoaming)))) (.Y (Math|Vector|BreakVector (* (Math|Vector|Normalize (- (stale _output_get_3) _returnvalue_2)) (Variables|Default|GetspeedRoaming)))) 0.0) _returnvalue_2) false false)
        (if (> _output_get 5.0)
          (Variables|Default|SetcurrentIntervalIdle 0.0)
          (bind _output_get_2 (Variables|Default|SetinitialTransform (Transformation|GetActorTransform)))
          (bind _output_get_3 (Variables|Default|SetNewLocation (+ (Variables|Default|GetinitialPosition) (Math|Vector|MakeVector (Math|Random|RandomFloatinRange -2e+02 2e+02) (Math|Random|RandomFloatinRange -2e+02 2e+02) 0.0))))
          (Variables|Default|SetfinalTransform (Math|Transform|MakeTransform _output_get_3 (.Rotation (Math|Transform|BreakTransform _output_get_2)) (.Scale (Math|Transform|BreakTransform _output_get_2)))))))))

(fn ConstructionScript)